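; Fire effect Blueprint that pairs a configurable particle system with an optional point light.
; The construction script applies the particle template and the light's visibility, intensity and radius.
; From BeginPlay, a timeline updates the "dir" particle parameter using either its oscillating vector or a fixed Direction, plus random X/Y jitter.
; Each update also passes the owner as VertSurfaceActor, activates the system and toggles smoke and distortion emitters.
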(event `self.ReceiveBeginPlay`
  (bind _particlesystem (`self.ParticleSystem`))
  (bind _returnvalue (`KismetMathLibrary.RandomFloatInRange` (`self.Random_Start_angle_min`) (`self.Random_Start_angle_max`)))
  (bind _returnvalue_2 (`KismetMathLibrary.MakeVector` _returnvalue _returnvalue))
  (`TimelineComponent.SetPlayRate` (`self.Timeline_0`) (`self.Oscil_Speed`))
  (bind (_direction _dir_vector) (`Timeline|Timeline_0`)
    (:`Update`
      (`ParticleSystemComponent.SetVectorParameter` _particlesystem "dir" (select `bool` (`self.oscillate`) :`false` (`KismetMathLibrary.Normal` (+ (`self.Direction`) _returnvalue_2)) :`true` (`KismetMathLibrary.Normal` (+ _dir_vector _returnvalue_2))))
      (`ParticleSystemComponent.SetActorParameter` _particlesystem "VertSurfaceActor" (`ActorComponent.GetOwner` (`self.ParticleSystem`)))
      (`ActorComponent.Activate` _particlesystem false)
      (`ParticleSystemComponent.SetEmitterEnable` (`self.ParticleSystem`) "smoke" (`self.Smoke_Emitter_Enable`))
      (`ParticleSystemComponent.SetEmitterEnable` (`self.ParticleSystem`) "Distortion" (`self.Distortion_Emittter_Enable`)))))

(fn `UserConstructionScript`
  (bind _pointlight (`self.PointLight`))
  ;[1 1 1] Light
  (`SceneComponent.SetVisibility` _pointlight (`self.Light`) false)
  (`LightComponent.SetIntensity` _pointlight (`self.Light_Intensity`))
  (`PointLightComponent.SetAttenuationRadius` _pointlight (`self.LightRadius`))
  (`ParticleSystemComponent.SetTemplate` (`self.ParticleSystem`) (`self.particle_fire`)))