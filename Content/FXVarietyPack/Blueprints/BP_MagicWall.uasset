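; A magic wall barrier that stays hidden and non-colliding until a character enters its trigger box.
; The first overlap by an M_CharacterBase, guarded by a one-shot flag, reveals the effect, enables collision and plays a shield sound and music track in 2D.
; The construction script passes the Color variable into the effect's color parameter.
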(event `self.ReceiveBeginPlay`
  (`SceneComponent.SetHiddenInGame` (`self.fx`) true false)
  (`PrimitiveComponent.SetCollisionEnabled` (`self.collider`) "NoCollision"))

(event `self.TriggerBox.OnComponentBeginOverlap`
  (params (OverlappedComponent :type "PrimitiveComponent Object Reference") (OtherActor :type "Actor Object Reference") (OtherComp :type "PrimitiveComponent Object Reference") (OtherBodyIndex :type Integer) (bFromSweep :type Boolean) (SweepResult :type "HitResult Structure (by ref)"))
  (cast `/Game/SHINTO_Content/Player/M_CharacterBase` OtherActor)
  (if (not (`self.TriggerStarted`))
    (set `self.TriggerStarted` true)
    (`SceneComponent.SetHiddenInGame` (`self.fx`) false false)
    (`PrimitiveComponent.SetCollisionEnabled` (`self.collider`) "QueryAndPhysics")
    (`GameplayStatics.PlaySound2D` "/Game/SHINTO_Content/Sound/SFX/WeaponSFX/570852__rafaelzimrp__magicshield_down.570852__rafaelzimrp__magicshield_down" 1.0 1.0 0.0 null null)
    (`GameplayStatics.PlaySound2D` "/Game/SHINTO_Content/Sound/SFX/Music/Japanese_Fantasy_Music_-_Honō_no_Megami__炎の女神_.Japanese_Fantasy_Music_-_Honō_no_Megami__炎の女神_" 1.0 1.0 0.0 null null)))

(fn `UserConstructionScript`
  (`parent.UserConstructionScript`)
  (`ParticleSystemComponent.SetVectorParameter` (`self.fx`) "color" (`KismetMathLibrary.Conv_LinearColorToVector` (`self.color`))))