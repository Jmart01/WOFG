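; BP_NavGuide is a navigation guide pawn that moves by AI toward a point on a checkpoint actor.
; BeginPlay caches the first NavGuide_CheckPoints actor after a short delay.
; GoToLoc converts that actor's second point to world space and calls AIMoveTo, printing debug text.
; GetCheckPoint looks unfinished: it searches for the nearest checkpoint from world origin but clears the reference instead of storing the result.
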(event `self.ReceiveBeginPlay`
  (`KismetSystemLibrary.Delay` 0.1)
  (bind _outactors (`GameplayStatics.GetAllActorsOfClass` "/Game/SHINTO_Content/Player/Navigation/NavGuide_CheckPoints.NavGuide_CheckPoints_C"))
  (set `self.NavGuide_Checkpoints` (`|GetArrayItem` _outactors)))

(event `GoToLoc`
  (bind _navguide_checkpoints (`self.NavGuide_Checkpoints`))
  (`KismetSystemLibrary.Delay` 0.2)
  (`/Engine/EditorBlueprintResources/StandardMacros.IsValid` _navguide_checkpoints
    (:`Is Valid`
      (`|AIMoveTo` self (`KismetMathLibrary.TransformLocation` (`self.GetTransform` _navguide_checkpoints) (`|GetArrayItem` (`/Game/SHINTO_Content/Player/Navigation/NavGuide_CheckPoints.Points` _navguide_checkpoints) 1)) null 5.0 true
        (:`then`
          _)
        (:`OnSuccess`
          _))
      (`KismetSystemLibrary.PrintString` "Hello"))
    (:`Is Not Valid`
      (`KismetSystemLibrary.PrintString` "Not Valid"))))

(fn `GetCheckPoint`
  (returns (CheckPoint :type "/Game/SHINTO_Content/Player/Navigation/NavGuide_CheckPoints Object Reference"))
  (bind _outactors (`GameplayStatics.GetAllActorsOfClass` (`GameplayStatics.GetObjectClass` (`self.NavGuide_Checkpoints`))))
  (`/Engine/EditorBlueprintResources/StandardMacros.IsValid` (`.ReturnValue` (`GameplayStatics.FindNearestActor` (0.0 0.0 0.0) _outactors))
    (:`Is Valid`
      (bind _output_get (set `self.NavGuide_Checkpoints` null))
      (return _output_get))
    (:`Is Not Valid`
      (`KismetSystemLibrary.PrintString` "Not valid to begin with"))))

(fn `UserConstructionScript`)