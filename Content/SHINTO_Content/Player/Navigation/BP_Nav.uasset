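; BP_Nav is a short-lived navigation actor that moves to the nearest point on a spline, then along it.
; Shortly after BeginPlay it takes the first Spline actor found and searches its points for the closest one.
; One timeline lerps it to that point; a second moves it by distance to the next point, starting a five-second countdown to self-destruction.
; StopMovement halts both timelines.
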(event `self.ReceiveBeginPlay`
  (`KismetSystemLibrary.Delay` 0.1)
  (bind _outactors (`GameplayStatics.GetAllActorsOfClass` "/Game/SHINTO_Content/Player/Navigation/Spline.Spline_C"))
  (set `self.SplineToUse` (`|GetArrayItem` _outactors))
  (set `self.StartLoc` (`self.K2_GetActorLocation`))
  (`self.GoToLoc`))

(event `GoToLoc`
  (bind _closestsplineindex (`self.ClosestSplineIndex`))
  (bind _spline (`/Game/SHINTO_Content/Player/Navigation/Spline.Spline` (`self.SplineToUse`)))
  (bind _spline_2 (`/Game/SHINTO_Content/Player/Navigation/Spline.Spline` (`self.SplineToUse`)))
  (for _index (range (+ (`SplineComponent.GetNumberOfSplinePoints` _spline_2) 1))
    (bind _returnvalue (`SplineComponent.GetLocationAtSplinePoint` _spline_2 _index "World"))
    (bind _returnvalue_2 (`KismetMathLibrary.Vector_Distance` (`self.K2_GetActorLocation` self) _returnvalue))
    (if (< _returnvalue_2 (`self.SmallestDist`))
      (bind _output_get (set `self.closestDist` _returnvalue))
      (set `self.ClosestSplineIndex` _index)
      (set `self.SmallestDist` _returnvalue_2)))
  (bind (_direction _starttospline) (`Timeline|Move to Spline` :!via `PlayFromStart` :!label _label)
    (:`Update`
      (`self.K2_SetActorLocation` (`KismetMathLibrary.VLerp` (`self.StartLoc`) _output_get _starttospline)))
    (:`Finished`
      (bind (_direction_2 _alongspline) (`Timeline|Move along Spline` :!via `PlayFromStart` :!label _label_2)
        (:`Update`
          (`self.K2_SetActorLocation` (`SplineComponent.GetLocationAtDistanceAlongSpline` _spline (`KismetMathLibrary.Lerp` (`SplineComponent.GetDistanceAlongSplineAtSplinePoint` _spline _closestsplineindex) (`SplineComponent.GetDistanceAlongSplineAtSplinePoint` _spline (+ _closestsplineindex 1)) _alongspline) "World"))
          (`KismetSystemLibrary.Delay` 5.0)
          (`self.K2_DestroyActor`))))))

(event `StopMovement`
  (`|ExecutionSequence`
    (:`then_0`
      (goto _label :!via `Stop`))
    (:`then_1`
      (goto _label_2 :!via `Stop`))))

(fn `UserConstructionScript`)