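; Player ability projectile that homes in on an AI-controlled character.
; A detection capsule collects overlapping characters with a MyAIController, locks onto the nearest within ClosestDistance, then destroys itself.
; Tick turns the projectile toward that target and sets its velocity forward at ProjectileSpeed.
; It destroys itself when its sphere overlaps the target; lifetime expiry only prints a debug message.
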(event `self.ReceiveBeginPlay`
  (`KismetSystemLibrary.Delay` (`self.LifeDuration`))
  (`KismetSystemLibrary.PrintString` "should delete"))

(event `self.Capsule.OnComponentBeginOverlap`
  (params (OverlappedComponent :type "PrimitiveComponent Object Reference") (OtherActor :type "Actor Object Reference") (OtherComp :type "PrimitiveComponent Object Reference") (OtherBodyIndex :type Integer) (bFromSweep :type Boolean) (SweepResult :type "HitResult Structure (by ref)"))
  (bind _targets (`self.Targets`))
  (bind _ascharacter (cast `Character` OtherActor))
  (bind _returnvalue (`AIBlueprintHelperLibrary.GetAIController` _ascharacter))
  (bind _asmy_aicontroller (cast `MyAIController` _returnvalue))
  (if (== _asmy_aicontroller _returnvalue)
    (`KismetArrayLibrary.Array_Add` _targets _ascharacter)
    (for _array_element _targets
      (bind _returnvalue_2 (`KismetMathLibrary.Vector_Distance` (`self.K2_GetActorLocation` _array_element) (`self.K2_GetActorLocation`)))
      (if (< _returnvalue_2 (`self.ClosestDistance`))
        (set `self.ClosestDistance` _returnvalue_2)
        (set `self.ClosestTarget` _array_element)
        (`ActorComponent.K2_DestroyComponent` (`self.Capsule`))))))

(event `self.ReceiveTick`
  (params (DeltaSeconds :type "Float (single-precision)"))
  (`/Engine/EditorBlueprintResources/StandardMacros.IsValid` (`self.ClosestTarget`)
    (:`Is Valid`
      (`self.K2_SetActorRotation` (`KismetMathLibrary.FindLookAtRotation` (`self.K2_GetActorLocation`) (`self.K2_GetActorLocation` (`self.ClosestTarget`))))
      (set `self.Velocity` (* (`self.GetActorForwardVector`) (`self.Projectile Speed`))))))

(event `self.SphereComp.OnComponentBeginOverlap`
  (params (OverlappedComponent :type "PrimitiveComponent Object Reference") (OtherActor :type "Actor Object Reference") (OtherComp :type "PrimitiveComponent Object Reference") (OtherBodyIndex :type Integer) (bFromSweep :type Boolean) (SweepResult :type "HitResult Structure (by ref)"))
  (if (== OtherActor (`self.ClosestTarget`))
    (`KismetSystemLibrary.PrintString` "should delete myself")
    (`self.K2_DestroyActor`)
    (else
      (`KismetSystemLibrary.PrintString` "is not closest target"))))

(fn `UserConstructionScript`)