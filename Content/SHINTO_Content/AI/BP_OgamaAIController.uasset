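; BP_OgamaAIController is the AI controller for the Ogama character, a child class that leaves nearly all behavior to its parent.
; Its only added logic is on ResumeAILogic, which calls the parent, clears SoulCombination and calls SetSoulCombo to set the combo again.
; BeginPlay, Possess and SetSoulCombo only forward to the parent, and a SetDeathProcess debug print sits unconnected.
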(event `self.ReceiveBeginPlay`
  (`parent.ReceiveBeginPlay`))

(event `self.ReceivePossess`
  (params (PossessedPawn :type "Pawn Object Reference"))
  (`parent.ReceivePossess` PossessedPawn))

(event `self.SetSoulCombo`
  (`parent.SetSoulCombo`))

(event `self.ResumeAILogic`
  (`parent.ResumeAILogic`)
  (`KismetArrayLibrary.Array_Clear` (`self.SoulCombination`))
  (`self.SetSoulCombo`))

(fn `UserConstructionScript`
  (`parent.UserConstructionScript`))