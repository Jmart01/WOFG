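; BP_KijikuiAI is the Blueprint for the Kijikui enemy AI character, which uses a snail attack animation and reacts to a quick-time event.
; BeginPlay replays a walk sound cue every second in an endless delay loop.
; The attack event slows the actor to half time dilation and plays the attack montage, with a separate event restoring normal speed.
; Passing the QTE stops the montage and destroys the actor.
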(event `self.ReceiveBeginPlay`
  (`AudioComponent.Play` (`self.Kijikui_Walk_Cue`) 0.0 :!label _label)
  (`KismetSystemLibrary.Delay` 1.0)
  (goto _label))

(event `play Attack Montage`
  (set `self.CustomTimeDilation` 0.5)
  (`|PlayMontage` (`self.Mesh`) "/Game/SHINTO_Content/AI/Kijikui_AI/Anims/Snail_Attk_Anim_Montage.Snail_Attk_Anim_Montage"))

(event `ResetTimeDilation`
  (set `self.CustomTimeDilation` 1.0))

(event `Player Passed QTE`
  (`AnimInstance.Montage_Stop` (`SkeletalMeshComponent.GetAnimInstance` (`self.Mesh`)) 0.0 null)
  (`self.K2_DestroyActor`))

(fn `UserConstructionScript`)