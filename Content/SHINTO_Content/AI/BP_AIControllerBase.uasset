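; AI controller base for the Kijikui enemy, giving each possessed pawn a random three-key "soul combo" for a quick-time input check.
; The combo is shown on the pawn; inputs found anywhere in it advance the visible progress, while others reset it.
; A third match stops the AI logic for a few seconds before rerunning the behavior tree.
; A separate event plays the death montage.
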(event `self.ReceiveBeginPlay`)

(event `self.ReceivePossess`
  (params (PossessedPawn :type "Pawn Object Reference"))
  (set `self.Possessed Pawn` PossessedPawn)
  (`parent.ReceivePossess` PossessedPawn)
  (`KismetSystemLibrary.Delay` 0.2)
  (bind _asbp_kijikui_ai (cast `/Game/SHINTO_Content/AI/Kijikui_AI/BP_KijikuiAI` (`self.Possessed Pawn`))
    (:`then`
      (set `self.PawnAsKijikuiBP` _asbp_kijikui_ai)
      (`self.SetSoulCombo`))
    (:`CastFailed`
      (`KismetSystemLibrary.PrintString` "Cast Fail"))))

(event `SetSoulCombo`
  ;[1 1 1] Sets the pawn's unique soul combo
  (for _ (range 3)
    (`KismetArrayLibrary.Array_Add` (`self.SoulCombination`) (`KismetArrayLibrary.Array_Random` (`self.Keys`))))
  (`/Game/SHINTO_Content/AI/Kijikui_AI/BP_KijikuiAI.SetComboKeyTexts` (`self.PawnAsKijikuiBP`) (`self.SoulCombination`)))

(event `CheckInputs`
  (params (`Player Input` :type "Key Structure" :default "None"))
  (bind _pawnaskijikuibp (`self.PawnAsKijikuiBP`))
  (bind _keyindex (`self.keyIndex`))
  ;[1 1 1] Checks Player Inputs to the Soul Combo
  (if (`KismetArrayLibrary.Array_Contains` (`self.SoulCombination`) `Player Input`)
    (`/Game/SHINTO_Content/AI/Kijikui_AI/BP_KijikuiAI.ChangeVisibility` _pawnaskijikuibp false _keyindex)
    (set `self.keyIndex` (+ _keyindex 1))
    (if (== _keyindex 3)
      (`self.PauseAILogic`))
    (else
      (set `self.keyIndex` 0)
      (`/Game/SHINTO_Content/AI/Kijikui_AI/BP_KijikuiAI.ChangeVisibility` _pawnaskijikuibp true 0)
      (`KismetSystemLibrary.PrintString` "failed QTE"))))

(event `self.SetDeathProcess`
  ;[1 1 1] Death
  (`AnimInstance.Montage_Play` (`SkeletalMeshComponent.GetAnimInstance` (`Character.Mesh` (`self.PawnAsKijikuiBP`))) "/Game/SHINTO_Content/AI/Kijikui_AI/Anims/SnailDeathJan30_Montage.SnailDeathJan30_Montage" 1.0 "MontageLength" 0.0 true))

(event `PauseAILogic`
  ;[1 1 1] Pauses and resumes ai logic
  (`BrainComponent.StopLogic` (`self.BrainComponent`) "")
  (`KismetSystemLibrary.Delay` 5.0)
  (`self.ResumeAILogic`))

(event `ResumeAILogic`
  ;[1 1 1] Pauses and resumes ai logic
  (`self.RunBehaviorTree` (`self.BehaviorTreeToUse`)))

(fn `UserConstructionScript`)