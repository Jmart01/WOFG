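; BP_OgamaAI is the Ogama enemy character, extending a parent AI Blueprint with its own montages and reactions.
; BeginPlay sets the attack montage; hit and death events play theirs, then respectively restart the controller's behavior tree or destroy controller and actor.
; JumpBack launches the character along world Y, and SetShouldPlayCharged returns a random bool.
; RotateAroundPlayer only prints, HopBack is empty, and orbit logic is disconnected.
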(event `JumpBack`
  (params (Distance :type "Float (double-precision)"))
  (bind (_returnvalue_x _returnvalue_y) (`KismetMathLibrary.BreakVector` (`CharacterMovementComponent.GetLastUpdateVelocity` (`self.CharacterMovement`))))
  (`KismetSystemLibrary.PrintString` "Jump Back Is Called")
  (`self.LaunchCharacter` (`KismetMathLibrary.MakeVector` 0.0 (* (+ _returnvalue_y Distance) -1.0) 40.0) true true))

(event `RotateAroundPlayer`
  (params (PlayerLocation :type "Vector Structure"))
  (`KismetSystemLibrary.PrintString` "Should rotate around character"))

(event `self.ReceiveBeginPlay`
  (set `self.AttackAnim` "/Game/SHINTO_Content/AI/Ogama_AI/Animations/Ogama_Attack_feb27_Montage.Ogama_Attack_feb27_Montage")
  (`KismetSystemLibrary.PrintString` "attack set")
  (set `self.DeathAnim` null)
  (`KismetSystemLibrary.PrintString` "Death Set")
  (set `self.HitAnim` null)
  (`KismetSystemLibrary.PrintString` "Hit set"))

(event `self.SetComboImages`
  (params (SoulCombo :type "Array of Key Structure (by ref)"))
  (`parent.SetComboImages` SoulCombo))

(event `self.Play Hit Montage`
  (`parent.Play Hit Montage`)
  (`|PlayMontage` (`self.Mesh`) "/Game/SHINTO_Content/AI/Ogama_AI/Animations/OgamaHitFeb26V4_Montage.OgamaHitFeb26V4_Montage"
    (:`OnCompleted`
      (`KismetSystemLibrary.Delay` 0.2)
      (bind _asbp_ogama_aicontroller (cast `/Game/SHINTO_Content/AI/BP_OgamaAIController` (`AIBlueprintHelperLibrary.GetAIController` self)))
      (`AIController.RunBehaviorTree` _asbp_ogama_aicontroller (`MyAIController.BehaviorTreeToUse` _asbp_ogama_aicontroller)))))

(event `self.Play Death Montage`
  (`parent.Play Death Montage`)
  (`|PlayMontage` (`self.Mesh`) "/Game/SHINTO_Content/AI/Ogama_AI/Animations/OgamaDeathFeb26_Montage.OgamaDeathFeb26_Montage"
    (:`OnCompleted`
      (`KismetSystemLibrary.Delay` 1.0)
      (`self.K2_DestroyActor` (`AIBlueprintHelperLibrary.GetAIController` self))
      (`self.K2_DestroyActor` self))))

(event `HopBack`)

(fn `Set Should Play Charged`
  (returns (Decision :type Boolean))
  (return (`KismetMathLibrary.RandomBool`)))

(fn `UserConstructionScript`)