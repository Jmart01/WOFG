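; AI controller for the Kijikui enemy that gives it a random soul combination of keys at the start of play.
; On BeginPlay it draws random picks from its Keys array, repeats allowed, making one fewer pick than the array holds.
; It passes the sequence to the possessed BP_KijikuiAI pawn to set its combo key texts.
; Unreachable leftover nodes reference Ogama_AI and a direct soul combination widget update.
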(event `self.ReceiveBeginPlay`
  (for _ (range (`KismetArrayLibrary.Array_LastIndex` (`self.Keys`)))
    (`KismetArrayLibrary.Array_Add` (`self.SoulCombination`) (`KismetArrayLibrary.Array_Random` (`self.Keys`))))
  (bind _asbp_kijikui_ai (cast `/Game/SHINTO_Content/AI/Kijikui_AI/BP_KijikuiAI` (`self.K2_GetPawn` self)))
  (`/Game/SHINTO_Content/AI/Kijikui_AI/BP_KijikuiAI.SetComboKeyTexts` _asbp_kijikui_ai (`self.SoulCombination`)))

(fn `UserConstructionScript`)