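; Ogama enemy AI character, a child Blueprint that sets its attack montage and extends parent combat events.
; Hits play a montage, then re-run the AI controller's behavior tree after a short delay; death stops slot animation and flags the anim Blueprint dead.
; JumpBack launches the character using world-Y velocity and distance, and charged attacks are chosen randomly.
; RotateAroundPlayer only prints, with its orbit math left unconnected.
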(event `JumpBack`
  (params (Distance :type "Float (double-precision)"))
  (bind (_returnvalue_x _returnvalue_y) (`KismetMathLibrary.BreakVector` (`CharacterMovementComponent.GetLastUpdateVelocity` (`self.CharacterMovement`))))
  (`KismetSystemLibrary.PrintString` "Jump Back Is Called")
  (`self.LaunchCharacter` (`KismetMathLibrary.MakeVector` 0.0 (* (+ _returnvalue_y Distance) -1.0) 40.0) true true))

(event `RotateAroundPlayer`
  (params (PlayerLocation :type "Vector Structure"))
  (`KismetSystemLibrary.PrintString` "Should rotate around character"))

(event `self.ReceiveBeginPlay`
  ;[1 1 1] Begin play
  (set `self.AttackAnim` "/Game/SHINTO_Content/AI/Ogama_AI/Animations/Ogama_Attack_feb27_Montage.Ogama_Attack_feb27_Montage")
  (`KismetSystemLibrary.PrintString` "attack set")
  (set `self.HitAnim` null)
  (`KismetSystemLibrary.PrintString` "Hit set"))

(event `self.SetComboImages`
  (params (SoulCombo :type "Array of Key Structure (by ref)"))
  ;[1 0.6468 0.06771] Set combo images
  (`parent.SetComboImages` SoulCombo))

(event `self.Play Hit Montage`
  ;[1 0 0.08316] plays hit and stuns for a little bit
  (`parent.Play Hit Montage`)
  (`|PlayMontage` (`self.Mesh`) "/Game/SHINTO_Content/AI/Ogama_AI/Animations/OgamaHitFeb26V4_Montage.OgamaHitFeb26V4_Montage"
    (:`OnCompleted`
      (`KismetSystemLibrary.Delay` 0.2)
      (bind _asbp_ogama_aicontroller (cast `/Game/SHINTO_Content/AI/BP_OgamaAIController` (`AIBlueprintHelperLibrary.GetAIController` self)))
      (`AIController.RunBehaviorTree` _asbp_ogama_aicontroller (`MyAIController.BehaviorTreeToUse` _asbp_ogama_aicontroller)))))

(event `self.Play Death Montage`
  (bind _returnvalue (`SkeletalMeshComponent.GetAnimInstance` (`self.Mesh`)))
  ;[0 0.05329 1] Death
  (`KismetSystemLibrary.PrintString` "Gets to Play death Montage in the ogama")
  (`AnimInstance.StopSlotAnimation` _returnvalue 0.25 "None")
  (bind _asogama_anim_bp (cast `/Game/SHINTO_Content/AI/Ogama_AI/Animations/Ogama_Anim_BP` _returnvalue)
    (:`then`
      (`/Game/SHINTO_Content/AI/Ogama_AI/Animations/Ogama_Anim_BP.SetDeadToTrue` _asogama_anim_bp))
    (:`CastFailed`
      (`KismetSystemLibrary.PrintString` "not the ogama anim bp"))))

(event `self.Set Hitbox Enabled`
  (`parent.Set Hitbox Enabled`))

(event `self.DestroyControllerPawn`
  ;[0 0.05329 1] Death
  (`parent.DestroyControllerPawn`))

(event `self.Set Hitbox Disabled`
  (`parent.Set Hitbox Disabled`))

(fn `Set Should Play Charged`
  (returns (Decision :type Boolean))
  (return (`KismetMathLibrary.RandomBool`)))

(fn `UserConstructionScript`)